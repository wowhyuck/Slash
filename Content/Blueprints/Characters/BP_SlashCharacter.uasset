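; Player character Blueprint that adds lock-on targeting, interaction, pause and quest log input to the Slash character.
; The LockOnTarget component redirects look input to target switching while locked, and its events change character state, rotation mode and walk speed.
; A forward sphere trace each tick caches an IInteractionInterface actor, whose interact message is broadcast as an objective ID.
; Input opens the pause menu, pausing the game, or creates a quest log widget.
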(event OnTargetLocked(LockOnTarget)
  (params (Target :type Targeting%20Helper%20Component%20Object%20Reference) (Socket :type Name :default "None"))
  (Variables|/Script/Engine.CharacterMovementComponent|SetbOrientRotationToMovement (Variables|Character|GetCharacterMovement) false)
  (Variables|Default|SetCharacterState "ECS_LockingOnTarget")
  (Variables|/Script/Engine.CharacterMovementComponent|SetMaxWalkSpeed (Variables|Character|GetCharacterMovement) 3e+02))

(event OnTargetUnlocked(LockOnTarget)
  (params (UnlockedTarget :type Targeting%20Helper%20Component%20Object%20Reference) (Socket :type Name :default "None"))
  (Variables|/Script/Engine.CharacterMovementComponent|SetbOrientRotationToMovement (Variables|Character|GetCharacterMovement) true)
  (Variables|Default|SetCharacterState "ECS_EquippedWeapon")
  (Variables|/Script/Engine.CharacterMovementComponent|SetMaxWalkSpeed (Variables|Character|GetCharacterMovement) 4.5e+02))

(event EventBeginPlay
  (Input|SetInputModeGameOnly (Game|GetPlayerController 0)))

(event EventTick
  (params (DeltaSeconds :type Float%20%28single-precision%29))
  (|CallParentFunction DeltaSeconds)
  (CallFunction|InteractTrace))

(event Input|ActionEvents|InputActionPause
  (params (Key :type Key%20Structure :default "None"))
  (bind _returnvalue (Game|GetPlayerController 0))
  (:Pressed
    (Utilities|IsValid (Variables|Default|GetPauseMenuReference)
      (:Is%20Valid
        _)
      (:Is%20Not%20Valid
        (bind _returnvalue_2 (UserInterface|CreateWidget "/Game/Blueprints/HUD/MenuHUD/WBP_PauseMenu.WBP_PauseMenu_C"))
        (Variables|Default|SetPauseMenuReference _returnvalue_2)))
    (Variables|/Script/Engine.PlayerController|SetbShowMouseCursor _returnvalue true)
    (Input|SetInputModeUIOnly _returnvalue (Variables|Default|GetPauseMenuReference) "DoNotLock")
    (UserInterface|Viewport|AddtoViewport (Variables|Default|GetPauseMenuReference) 0)
    (Game|SetGamePaused true)))

(event Input|ActionEvents|InputActionLockOn
  (params (Key :type Key%20Structure :default "None"))
  (:Pressed
    (Class|LockonTargetComponent|EnableTargeting (Variables|Default|GetLockOnTarget))))

(event Input|ActionEvents|InputActionInteract
  (params (Key :type Key%20Structure :default "None"))
  (:Pressed
    (bind _lookatactor (Variables|Default|GetLookAtActor)
      (:then
        (bind _objectiveid (Class|IInteractionInterface|Interactwith(Message) _lookatactor))
        (Default|CallOnObjectiveIDCalled _objectiveid))
      (:else))))

(event Input|ActionEvents|InputActionQuestLog
  (params (Key :type Key%20Structure :default "None"))
  (:Pressed
    (bind _returnvalue (UserInterface|CreateWidget "/Game/Blueprints/HUD/QuestHUD/WBP_QuestLog.WBP_QuestLog_C"))
    (UserInterface|Viewport|AddtoViewport _returnvalue 0)))

(event Input|AxisEvents|InputAxisTurn
  (params (AxisValue :type Float%20%28single-precision%29))
  (if (Class|LockonTargetComponent|IsTargetLocked (Variables|Default|GetLockOnTarget))
    (Class|LockonTargetComponent|SwitchTargetYaw (Variables|Default|GetLockOnTarget) AxisValue)
    (else
      (Pawn|Input|AddControllerYawInput AxisValue))))

(event Input|AxisEvents|InputAxisLookUp
  (params (AxisValue :type Float%20%28single-precision%29))
  (if (Class|LockonTargetComponent|IsTargetLocked (Variables|Default|GetLockOnTarget))
    (Class|LockonTargetComponent|SwitchTargetPitch (Variables|Default|GetLockOnTarget) (* AxisValue -1.0))
    (else
      (Pawn|Input|AddControllerPitchInput AxisValue))))

(fn ConstructionScript)

(fn InteractTrace
  (bind _returnvalue (Transformation|GetActorLocation))
  (bind _outhit (Collision|SphereTraceByChannel _returnvalue (+ _returnvalue (* (Transformation|GetActorForwardVector) 1e+02)) 2e+01 "TraceTypeQuery2" false (Utilities|Array|MakeArray (Components|GetOwner)) "None"))
  (if true
    (if (Utilities|DoesObjectImplementInterface (.HitActor (Collision|BreakHitResult _outhit)) "/Game/Blueprints/Interfaces/IInteractionInterface.IInteractionInterface_C")
      (bind _output_get (Variables|Default|SetLookAtActor (.HitActor (Collision|BreakHitResult _outhit))))
      (Class|IInteractionInterface|Lookat(Message) _output_get)
      (else
        (Variables|Default|SetLookAtActor 0)))
    (else
      (Variables|Default|SetLookAtActor 0))))