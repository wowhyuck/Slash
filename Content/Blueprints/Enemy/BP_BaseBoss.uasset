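; BP_BaseBoss is a base boss enemy that shows an on-screen boss health bar during the encounter.
; The first PawnSensing sighting of any pawn creates a WBP_BossHealthBar, sets its boss name and adds it to the viewport, guarded by a one-time flag.
; GetHit calls the parent implementation, then updates the bar from the Attributes health ratio, or removes it when the boss is dead.
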(event OnSeePawn(PawnSensing)
  (params (Pawn :type Pawn%20Object%20Reference))
  ;[1 1 1] 보스가 플레이어 볼 때, BossHealthBar Widget 띄우기
  (if (not (Variables|Default|GetbSeePawn))
    (Variables|Default|SetbSeePawn true)
    (bind _returnvalue (UserInterface|CreateWidget "/Game/Blueprints/HUD/WBP_BossHealthBar.WBP_BossHealthBar_C"))
    (bind _output_get (Variables|Default|SetBossHealthBar _returnvalue))
    (Rendering|Components|TextRender|SetText (Variables|/Game/Blueprints/HUD/WBP_BossHealthBar.WBP_BossHealthBar_C|GetBossName _returnvalue) (Utilities|Text|ToText(Name) (Variables|Default|GetBossName)))
    (UserInterface|Viewport|AddtoViewport _output_get 0)))

(event EventGetHit
  (params (ImpactPoint :type Vector%20%28by%20ref%29 :default "0, 0, 0") (Hitter :type Actor%20Object%20Reference))
  (bind _attributes (Variables|Default|GetAttributes))
  ;[1 1 1] 보스가 피격 당할 때, BossHealthBar SetPercent / 죽었을 때, Remove from Parent
  (|CallParentFunction ImpactPoint Hitter)
  (if (Variables|Default|GetbDead)
    (Widget|RemovefromParent (Variables|Default|GetBossHealthBar))
    (else
      (bind _bosshealthbar (Variables|Default|GetBossHealthBar)
        (:then
          (Progress|SetPercent (Variables|/Game/Blueprints/HUD/WBP_BossHealthBar.WBP_BossHealthBar_C|GetHealthBar _bosshealthbar) (/ (Variables|/Script/Slash.AttributeComponent|GetHealth _attributes) (Variables|/Script/Slash.AttributeComponent|GetMaxHealth _attributes))))
        (:else)))))

(event Collision|EventActorBeginOverlap
  (params (OtherActor :type Actor%20Object%20Reference)))

(event EventTick
  (params (DeltaSeconds :type Float%20%28single-precision%29)))

(fn ConstructionScript)