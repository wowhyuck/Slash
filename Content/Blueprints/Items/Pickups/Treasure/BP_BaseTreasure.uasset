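; Base treasure pickup actor that spins steadily around yaw and holds quest-tracking logic.
; On overlap with BP_SlashCharacter, it unbinds an event from OnItemReceived, looks up its QuestID row in the QuestList data table and stores it.
; It then seeds TaskProgress with a zero count for each task's item ID.
; OnQuestItemReceived only prints the received item ID and does not update progress.
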(event EventBeginPlay)

(event Collision|EventActorBeginOverlap
  (params (OtherActor :type Actor%20Object%20Reference))
  (bind _asbp_slash_character (Utilities|Casting|CastToBP_SlashCharacter OtherActor))
  (EventDispatchers|UnbindEventfromOnItemReceived _asbp_slash_character (EventDispatchers|CreateEvent :!event OnQuestItemReceived))
  (bind _returnvalue (Utilities|GetDataTableRow "/Game/Quest/QuestList.QuestList" (Variables|Default|GetQuestID))
    (:then
      (bind _output_get (Variables|Default|SetQuestData _returnvalue))
      (for _array_element (.Tasks (Utilities|Struct|BreakFQuest _output_get))
        (Utilities|Map|Add (Variables|Default|GetTaskProgress) (.ItemID (Utilities|Struct|BreakFTask _array_element)) 0)))))

(event EventTick
  (params (DeltaSeconds :type Float%20%28single-precision%29))
  (Class|Actor|AddActorWorldRotation (Math|Rotator|MakeRotator 0.0 0.0 (* DeltaSeconds 9e+01))))

(fn ConstructionScript)

(fn OnQuestItemReceived
  (params (ItemID :type Name))
  (Development|PrintString (Utilities|String|ToString(Name) ItemID)))