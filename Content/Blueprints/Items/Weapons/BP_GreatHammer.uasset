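; Great hammer weapon Blueprint that can shatter and scatter Chaos destructible objects at a given location.
; CreateFields applies a radial external cluster strain with no falloff to break clusters, then a radial linear force to push pieces outward from that point.
; The force field passes through a metadata filter.
; OnQuestItemReceived only prints the item ID, while BeginPlay and the construction script are empty.
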(event EventBeginPlay)

(event EventCreateFields
  (params (FieldLocation :type Vector%20%28by%20ref%29 :default "0, 0, 0"))
  (bind _fieldsystem (Variables|Default|GetFieldSystem))
  (Class|FieldSystemComponent|ApplyPhysicsField _fieldsystem true "Field_ExternalClusterStrain" 0 (Field|SetRadialFalloff (Variables|Default|GetRadialFalloff) 5e+05 0.8 1.0 0.0 2e+02 FieldLocation "Field_FallOff_None"))
  (Class|FieldSystemComponent|ApplyPhysicsField _fieldsystem true "Field_LinearForce" (Variables|Default|GetFieldSystemMetaDataFilter) (Field|SetRadialVector (Variables|Default|GetRadialVector) 5e+04 FieldLocation)))

(fn ConstructionScript)

(fn OnQuestItemReceived
  (params (ItemID :type Name))
  (Development|PrintString (Utilities|String|ToString(Name) ItemID)))