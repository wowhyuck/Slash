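; BP_NPC is a quest-giving NPC that shows a widget on overlap and opens a dialogue when interacted with.
; Its widget starts hidden and toggles with actor begin and end overlap, with no filter on the overlapping actor.
; Interact looks up the QuestRef data table row and, if found, creates a WBP_Dialogue with the quest data and ID, then adds it to the viewport.
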(event EventBeginPlay
  (|CallParentFunction)
  (Rendering|SetVisibility (Variables|Default|GetWidget) false false))

(event EventTick
  (params (DeltaSeconds :type Float%20%28single-precision%29)))

(event Collision|EventActorBeginOverlap
  (params (OtherActor :type Actor%20Object%20Reference))
  (Rendering|SetVisibility (Variables|Default|GetWidget) true false))

(event Collision|EventActorEndOverlap
  (params (OtherActor :type Actor%20Object%20Reference))
  (Rendering|SetVisibility (Variables|Default|GetWidget) false false))

(fn ConstructionScript)

(fn Interact
  (bind _questref (LocalVariables|GetQuestRef))
  (bind _returnvalue (Utilities|GetDataTableRow (.datatable _questref) (.rowname _questref))
    (:then
      (bind _returnvalue_2 (Game|ConstructObjectfromClass (Game|GetPlayerController 0) "/Game/Blueprints/HUD/QuestHUD/WBP_Dialogue.WBP_Dialogue_C" _returnvalue (.rowname _questref)))
      (UserInterface|Viewport|AddtoViewport _returnvalue_2 0)
      (return "None"))))