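; Base breakable Blueprint, built on a Geometry Collection with a capsule, for objects that can be hit and shattered.
; GetHit plays a pot-break sound at the impact point, then passes the hit to the parent implementation.
; When Chaos reports a break, the capsule stops blocking pawns and a short lifespan is set to remove the actor.
; BeginPlay prints a debug string and reports an AI noise event at the actor's location.
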(event OnChaosBreakEvent(GeometryCollection)
  (params (BreakEvent :type Chaos%20Break%20Event%20Structure%20%28by%20ref%29))
  (Actor|SetLifeSpan 3.0)
  (Collision|SetCollisionResponsetoChannel (Variables|Default|GetCapsule) "ECC_Pawn" "ECR_Ignore"))

(event EventBeginPlay
  (Development|PrintString "Breakable Begin")
  (Class|AISenseHearing|ReportNoiseEvent (Transformation|GetActorLocation) 1.0 self 0.0 "None"))

(event Collision|EventActorBeginOverlap
  (params (OtherActor :type Actor%20Object%20Reference)))

(event EventTick
  (params (DeltaSeconds :type Float%20%28single-precision%29)))

(event EventGetHit
  (params (ImpactPoint :type Vector%20%28by%20ref%29 :default "0, 0, 0") (Hitter :type Actor%20Object%20Reference))
  (Audio|PlaySoundatLocation "/Game/Assets/Audio/MetaSounds/SFX_PotBreak.SFX_PotBreak" ImpactPoint "0, 0, 0" 1.0 1.0 0.0 0 0 0 0)
  (|CallParentFunction ImpactPoint Hitter))

(fn ConstructionScript)